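; Effect spawner Blueprint that repeatedly creates a particle system, named as an explosion, at random points inside its Box component.
; BeginPlay starts SpawnEmmiter, a custom event that calls itself after each spawn, looping with a random delay while ActiveEmmiter is true.
; Each spawned system gets a random color from RandomCollorValues through its ColorUsarParam variable.
; The flag is checked before the delay, so a pending spawn still fires after it turns false.
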(event Custom|SpawnEmmiter
  (bind _box (Variables|Default|GetBox))
  (if (Variables|Default|GetActiveEmmiter)
    (Utilities|FlowControl|Delay (Math|Random|RandomFloatinRange 1.0 3.0))
    (bind _returnvalue (Niagara|SpawnSystematLocation (Variables|Default|GetSystem%20Template) (Math|Random|RandomPointinBoundingBox (Transformation|GetWorldLocation _box) (Variables|/Script/Engine.BoxComponent|GetBoxExtent _box))))
    (Niagara|SetNiagaraVariable(LinearColor) _returnvalue "ColorUsarParam" (Utilities|Array|Get(acopy) (Variables|Default|GetRandomCollorValues) (Math|Random|RandomIntegerinRange 0 7)))
    (CallFunction|SpawnEmmiter)))

(event EventBeginPlay
  (CallFunction|SpawnEmmiter))

(fn ConstructionScript)